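; GamePlayingState spawns waves of Goblin actors around the player during play.
; BeginPlay starts a looping timer that calls SpawnGoblinFunc every few seconds, spawning a random-sized batch each time.
; Each goblin gets a random X/Y offset converted from the player character's local space, so spawns always land in the forward-right quadrant at a distance, at the player's origin height.
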(event `self.ReceiveBeginPlay`
  (`KismetSystemLibrary.K2_SetTimer` null "SpawnGoblinFunc" 5.0 true))

(event `self.ReceiveTick`
  (params (DeltaSeconds :type "Float (single-precision)")))

(fn `SpawnGoblinFunc`
  (for _ (range (+ (`KismetMathLibrary.RandomIntegerInRange` 1 8) 1))
    (`|SpawnActorFromClass` "/Game/Characters/Goblin.Goblin_C" (`KismetMathLibrary.Conv_VectorToTransform` (`KismetMathLibrary.TransformLocation` (`self.GetTransform` (`GameplayStatics.GetPlayerCharacter` 0)) (`KismetMathLibrary.MakeVector` (`KismetMathLibrary.RandomFloatInRange` 750.0 1500.0) (`KismetMathLibrary.RandomFloatInRange` 750.0 1500.0)))) "Undefined" "MultiplyWithRoot" null null)))

(fn `UserConstructionScript`)